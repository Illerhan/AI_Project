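; BP_bullet is a projectile actor that destroys itself on hit and affects destructible actors and third-person characters.
; Destructibles take random damage at the impact point, pushed opposite the surface normal.
; Characters have Life negated rather than reduced by damage, then get a delayed-removal lifespan if it is zero or below.
; Both branches print a separately written random damage roll, which need not match the effect applied.
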(event `self.ReceiveBeginPlay`)

(event `self.ReceiveHit`
  (params (MyComp :type "PrimitiveComponent Object Reference") (Other :type "Actor Object Reference") (OtherComp :type "PrimitiveComponent Object Reference") (bSelfMoved :type Boolean) (HitLocation :type "Vector Structure") (HitNormal :type "Vector Structure") (NormalImpulse :type "Vector Structure") (Hit :type "HitResult Structure (by ref)"))
  (bind (_bblockinghit _binitialoverlap _time _distance _location _impactpoint _normal _impactnormal _physmat _hitactor) (`GameplayStatics.BreakHitResult` Hit))
  (bind _returnvalue (`KismetMathLibrary.RandomFloatInRange` 0.5 3.0))
  (`|ExecutionSequence`
    (:`then_0`
      (`self.K2_DestroyActor`)
      (bind _asdestructible_actor (cast `DestructibleActor` _hitactor))
      (`DestructibleComponent.ApplyDamage` (`DestructibleActor.DestructibleComponent` _asdestructible_actor) _returnvalue _impactpoint (* _impactnormal -1.0) 0.0)
      (`KismetSystemLibrary.PrintText` (`|FormatText` "Hit {actor} - {damage} Damages" (`KismetTextLibrary.Conv_StringToText` (`KismetStringLibrary.Conv_ObjectToString` _hitactor)) _returnvalue)))
    (:`then_1`
      (bind _asbp_third_person_character (cast `/Game/ThirdPerson/Blueprints/BP_ThirdPersonCharacter` _hitactor))
      (bind _output_get (set `/Game/ThirdPerson/Blueprints/BP_ThirdPersonCharacter.Life` (- 0.0 (`/Game/ThirdPerson/Blueprints/BP_ThirdPersonCharacter.Life` _asbp_third_person_character)) _asbp_third_person_character))
      (`KismetSystemLibrary.PrintText` (`|FormatText` "Hit {actor} - {damage} Damages" (`KismetTextLibrary.Conv_StringToText` (`KismetStringLibrary.Conv_ObjectToString` _hitactor)) _returnvalue))
      (if (<= _output_get 0.0)
        (`self.SetLifeSpan` _asbp_third_person_character 15.0)))))

(fn `UserConstructionScript`)